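; Player character Blueprint with Enhanced Input movement, jumping and camera look, where yaw turns the controller and pitch rotates the CameraDistance component.
; BeginPlay adds the input mapping context and HUD, while P or Escape runs the pause-menu logic.
; E messages overlapping actors that implement BPI_interact, and F prints wood and stone counts for testing.
; A delayed Tick steadily drains and prints health, destroying the player at zero.
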(event `Key|P`
  (params (Key :type "Key Structure"))
  (bind _returnvalue (`GameplayStatics.GetPlayerController` 0))
  (bind _returnvalue_2 (`GameplayStatics.GetPlayerController` 0))
  ;[0 0 0] Pause menu
  (:`Pressed`
    (if (not (`self.Is pause menu open`)) :!label _label
      (bind _returnvalue_3 (`|CreateWidget` "/Game/Player_controller_stuff/Pause_menu.Pause_menu_C" (`GameplayStatics.GetPlayerController` 0)))
      (bind _output_get (set `self.pause menu widget` _returnvalue_3))
      (`UserWidget.AddToViewport` _output_get 0)
      (`WidgetBlueprintLibrary.SetInputMode_GameAndUIEx` _returnvalue_2 null)
      (set `PlayerController.bShowMouseCursor` true _returnvalue)
      (`GameplayStatics.SetGamePaused` true)
      (else
        (set `self.Is pause menu open` false)
        (`Widget.RemoveFromParent` (`self.pause menu widget`))
        (`WidgetBlueprintLibrary.SetInputMode_GameOnly` _returnvalue_2)
        (set `PlayerController.bShowMouseCursor` false _returnvalue)
        (`GameplayStatics.SetGamePaused` false)))))

(event `Key|Escape`
  (params (Key :type "Key Structure"))
  ;[0 0 0] Pause menu
  (:`Pressed`
    (goto _label)))

(event `HUD`
  ;[0 0 0] HUD
  (bind _returnvalue (`|GenericCreateObject` "/Game/Player_controller_stuff/HUD.HUD_C"))
  (`UserWidget.AddToViewport` _returnvalue 0))

(event `self.ReceiveBeginPlay`
  ;[0 0 0] event begin play
  (`|ExecutionSequence`
    (:`then_0`
      (`self.mapping context`))
    (:`then_1`
      (`self.HUD`))))

(event `mapping context`
  ;[0 0 0] mapping context
  (bind _asplayer_controller (cast `PlayerController` (`self.GetController`)))
  (bind _returnvalue (pcsubsystem `EnhancedInputLocalPlayerSubsystem` _asplayer_controller))
  (`/Engine/EditorBlueprintResources/StandardMacros.IsValid` _returnvalue
    (:`Is Valid`
      (`EnhancedInputSubsystemInterface.AddMappingContext` _returnvalue "/Game/Player_controller_stuff/Input_action/IMC_player.IMC_player" 0 (struct)))))

(event `EnhancedInput|/Game/Player_controller_stuff/Input_action/Ia_jump`
  (params (ActionValue :type Boolean) (ElapsedSeconds :type "Float (double-precision)") (TriggeredSeconds :type "Float (double-precision)") (InputAction :type "InputAction Object Reference" :default "/Game/Player_controller_stuff/Input_action/Ia_jump.Ia_jump"))
  ;[0 0 0] Jumping
  (:`Triggered`
    (`self.Jump`))
  (:`Completed`
    (`self.StopJumping`)))

(event `EnhancedInput|/Game/Player_controller_stuff/Input_action/Ia_moving`
  (params (ActionValue :type "Vector2D Structure") (ElapsedSeconds :type "Float (double-precision)") (TriggeredSeconds :type "Float (double-precision)") (InputAction :type "InputAction Object Reference" :default "/Game/Player_controller_stuff/Input_action/Ia_moving.Ia_moving"))
  (bind (_returnvalue_roll _returnvalue_pitch _returnvalue_yaw) (`KismetMathLibrary.BreakRotator` (`self.GetControlRotation`)))
  (bind (_returnvalue_roll_2 _returnvalue_pitch_2 _returnvalue_yaw_2) (`KismetMathLibrary.BreakRotator` (`self.GetControlRotation`)))
  ;[0 0 0] Movment
  (:`Triggered`
    (`self.AddMovementInput` (`KismetMathLibrary.GetRightVector` (`KismetMathLibrary.MakeRotator` _returnvalue_roll_2 0.0 _returnvalue_yaw_2)) ActionValue_X)
    (`self.AddMovementInput` (`KismetMathLibrary.GetForwardVector` (`KismetMathLibrary.MakeRotator` 0.0 0.0 _returnvalue_yaw)) ActionValue_Y)))

(event `EnhancedInput|/Game/Player_controller_stuff/Input_action/Ia_look`
  (params (ActionValue :type "Vector2D Structure") (ElapsedSeconds :type "Float (double-precision)") (TriggeredSeconds :type "Float (double-precision)") (InputAction :type "InputAction Object Reference" :default "/Game/Player_controller_stuff/Input_action/Ia_look.Ia_look"))
  ;[0 0 0] camera
  (:`Triggered`
    (`self.AddControllerYawInput` ActionValue_X)
    (`SceneComponent.K2_AddLocalRotation` (`self.camera distance`) (`KismetMathLibrary.MakeRotator` 0.0 ActionValue_Y) false false)))

(event `Key|E`
  (params (Key :type "Key Structure"))
  ;[0 0 0] interact
  (:`Pressed`
    (for _array_element (`self.GetOverlappingActors` null)
      (if (`KismetSystemLibrary.DoesImplementInterface` _array_element "/Game/Player_controller_stuff/BPI_interact.BPI_interact_C")
        (message `/Game/Player_controller_stuff/BPI_interact.interact` _array_element)))))

(event `Key|F`
  (params (Key :type "Key Structure"))
  ;[0.4635 0 0.02563] material ammount test
  (:`Pressed`
    (`KismetSystemLibrary.PrintString` (`KismetStringLibrary.Conv_IntToString` (`self.num_wood`)) true true (struct :`R` 0.21 :`G` 0.073356 :`A` 1.0))
    (`KismetSystemLibrary.PrintString` (`KismetStringLibrary.Conv_IntToString` (`self.num_stone`)) true true (struct :`R` 0.197917 :`G` 0.197917 :`B` 0.197917 :`A` 1.0))))

(event `self.ReceiveTick`
  (params (DeltaSeconds :type "Float (single-precision)"))
  ;[0.1094 0 0] Health rot
  (`KismetSystemLibrary.Delay` 1.0)
  (set `self.Health` (- (`self.Health`) 3))
  (`KismetSystemLibrary.PrintString` (`KismetStringLibrary.Conv_IntToString` (`self.Health`)))
  (if (<= (`self.Health`) 0)
    (`self.K2_DestroyActor`)))

(fn `UserConstructionScript`)