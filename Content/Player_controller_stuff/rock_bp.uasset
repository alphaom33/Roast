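; Rock actor that the player can mine through an Interact event, yielding a stone pickup.
; Each interaction prints the current rock health to screen, then reduces it by one.
; When health reaches zero or below, the rock destroys itself and spawns a Bp_stone_pickup at its location.
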(event `/Game/Player_controller_stuff/BPI_interact.interact`
  (`KismetSystemLibrary.PrintString` (`KismetStringLibrary.Conv_IntToString` (`self.rock_health`)))
  (set `self.rock_health` (- (`self.rock_health`) 1))
  (if (<= (`self.rock_health`) 0)
    (`self.K2_DestroyActor`)
    (`|SpawnActorFromClass` "/Game/Player_controller_stuff/Bp_stone_pickup.Bp_stone_pickup_C" (`KismetMathLibrary.Conv_VectorToTransform` (`self.K2_GetActorLocation`)) "Undefined" "MultiplyWithRoot" null null)))

(fn `UserConstructionScript`)